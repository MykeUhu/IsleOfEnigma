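; BP_UhuPlayerController is a player controller that provides multiplayer text chat.
; On BeginPlay the local controller creates the WBP_ChatPanel widget, and Tick focuses its input box while the IA_EnterChat action is active.
; Serv_Submit loops over the GameState PlayerArray and calls OC_UpdateChat on each player's controller, which passes the sender name and message to that controller's chat panel.
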(event `self.ReceiveBeginPlay`
  (`self.Show Chat`))

(event `self.ReceiveTick`
  (params (DeltaSeconds :type "Float (single-precision)"))
  (if (`|GetInputActionValue`)
    (bind _wbp_chatpanel (`self.WBP_ChatPanel`)
      (:`then`
        (`Widget.SetKeyboardFocus` (`/Game/Main/Chat/Widget/WBP_ChatPanel.ChatInputBox` _wbp_chatpanel)))
      (:`else`))))

(event `Serv_Submit`
  (params (PlayerName :type Text) (ChatMessage :type Text))
  (for _array_element (`GameStateBase.PlayerArray` (`GameplayStatics.GetGameState`))
    (bind _asbp_uhu_player_controller (cast `/Game/Main/Blueprints/Player/BP_UhuPlayerController` (`PlayerState.GetPlayerController` _array_element)))
    (`self.OC_UpdateChat` _asbp_uhu_player_controller PlayerName ChatMessage)))

(event `OC_UpdateChat`
  (params (PlayerName :type Text) (ChatMessage :type Text))
  (bind _wbp_chatpanel (`self.WBP_ChatPanel`)
    (:`then`
      (`/Game/Main/Chat/Widget/WBP_ChatPanel.Update_Chat` _wbp_chatpanel PlayerName ChatMessage))
    (:`else`)))

(fn `Show Chat`
  (if (`self.IsLocalPlayerController`)
    (bind _returnvalue (`|CreateWidget` "/Game/Main/Chat/Widget/WBP_ChatPanel.WBP_ChatPanel_C" self))
    (bind _output_get (set `self.WBP_ChatPanel` _returnvalue))
    (`UserWidget.AddToViewport` _output_get 0)))

(fn `UserConstructionScript`)